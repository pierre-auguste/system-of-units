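; Abstract button actor with a colored button component and a text display for showing a value.
; An owner registers itself and an ID through RegisterButton, and UpdateValueRender sets the displayed text.
; The construction script tints the button through a dynamic M_Color material instance using ButtonColor.
; BeginPlay prints a red on-screen warning if the owner lacks SOU_HasButtonInterface; press handling is absent here.
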(event `self.ReceiveBeginPlay`
  (if (not (`KismetSystemLibrary.DoesImplementInterface` (`self.ButtonOwner`) "/Game/SOU/Blueprints/Interfaces/SOU_HasButtonInterface.SOU_HasButtonInterface_C"))
    (`KismetSystemLibrary.PrintString` (`KismetStringLibrary.Concat_StrStr` (`KismetSystemLibrary.GetDisplayName` self) " has no owner or the interface is not set") true true (struct :`R` 0.8 :`A` 1.0) 10.0)))

(event `UpdateValueRender`
  (params (NewText :type Text))
  (`TextRenderComponent.K2_SetText` (`self.ValueRender`) NewText))

(event `/Game/SOU/Blueprints/Interfaces/SOU_ButtonInterface.RegisterButton`
  (params (ButtonOwner :type "Actor Object Reference") (Id :type Integer))
  (set `self.ButtonOwner` ButtonOwner)
  (set `self.ButtonId` Id))

(fn `UserConstructionScript`
  (bind _returnvalue (`PrimitiveComponent.CreateDynamicMaterialInstance` (`self.Button`) 0 "/Game/SOU/Materials/M_Color.M_Color" "None"))
  (`MaterialInstanceDynamic.SetVectorParameterValue` _returnvalue "Color" (`self.ButtonColor`)))