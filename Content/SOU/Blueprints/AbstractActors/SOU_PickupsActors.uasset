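; Base pickup actor that can be grabbed and released by VR motion controllers.
; Pickup disables mesh physics, attaches the actor to the given component and records it as the right or left grabbed item on SOU_VRPawn, based on MotionSource.
; Drop detaches it in world space and sets physics simulation from the GameState's WorldGravity flag, so released items only simulate when that flag is on.
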(event `/Game/SOU/Blueprints/Interfaces/SOU_PickupsInterface.Pickup`
  (params (MotionControlle :type "MotionControllerComponent Object Reference") (AttacheTo :type "SceneComponent Object Reference"))
  (`PrimitiveComponent.SetSimulatePhysics` (`self.StaticMeshComponent`) false)
  (`SceneComponent.K2_AttachToComponent` (`self.K2_GetRootComponent`) AttacheTo "None" "KeepWorld" "KeepWorld" "KeepWorld" true)
  (bind _assou_vrpawn (cast `/Game/SOU/Chars/Player/SOU_VRPawn` (`ActorComponent.GetOwner` MotionControlle))
    (:`then`
      (if (== (`MotionControllerComponent.MotionSource` MotionControlle) "Right")
        (set `/Game/SOU/Chars/Player/SOU_VRPawn.GrabbedItemRight` self _assou_vrpawn)
        (else
          (set `/Game/SOU/Chars/Player/SOU_VRPawn.GrabbedItemLeft` self _assou_vrpawn))))
    (:`CastFailed`
      (`KismetSystemLibrary.PrintString` "SOU_PickupActory failed to cast to SOU_VRPAwn" true true (struct :`R` 1.0 :`A` 1.0) 5.0))))

(event `/Game/SOU/Blueprints/Interfaces/SOU_PickupsInterface.Drop`
  (bind _assou_game_state (cast `/Game/SOU/SOU_GameState` (`GameplayStatics.GetGameState`))
    (:`then`
      (`PrimitiveComponent.SetSimulatePhysics` (`self.StaticMeshComponent`) (`/Game/SOU/SOU_GameState.WorldGravity` _assou_game_state))
      (`self.K2_DetachFromActor` "KeepWorld" "KeepWorld" "KeepWorld"))
    (:`CastFailed`
      (`KismetSystemLibrary.PrintString` "PickupActor failed to cast to GameState" true true (struct :`R` 1.0 :`A` 1.0) 10.0))))

(fn `UserConstructionScript`)