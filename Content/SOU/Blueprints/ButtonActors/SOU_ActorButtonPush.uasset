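; SOU_ActorButtonPush is a momentary push button that the VR pawn triggers by overlapping its capsule.
; On overlap it sets IsActivated, refreshes the value render and sends the button ID with a true value to ButtonOwner.
; It animates the button mesh in and back out along local X using MoveComponentTo and delays.
; IsActivated blocks retriggering until the cycle ends, when it resets without messaging the owner.
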(event `self.Capsule.OnComponentBeginOverlap`
  (params (OverlappedComponent :type "PrimitiveComponent Object Reference") (OtherActor :type "Actor Object Reference") (OtherComp :type "PrimitiveComponent Object Reference") (OtherBodyIndex :type Integer) (bFromSweep :type Boolean) (SweepResult :type "HitResult Structure (by ref)"))
  (bind _button (`self.Button`))
  (bind _button_2 (`self.Button`))
  (bind _returnvalue (`SceneComponent.GetRelativeTransform` _button))
  (bind _returnvalue_2 (`SceneComponent.GetRelativeTransform` _button_2))
  (if (and (not (`self.isActivated`)) (== (`GameplayStatics.GetObjectClass` OtherActor) "/Game/SOU/Chars/Player/SOU_VRPawn.SOU_VRPawn_C"))
    (bind _output_get (set `self.isActivated` true))
    (`self.UpdateValueRender` (`KismetTextLibrary.Conv_BoolToText` _output_get))
    (message `/Game/SOU/Blueprints/Interfaces/SOU_HasButtonInterface.ReceiveButtonValue` (`self.ButtonOwner`) (`self.ButtonId`) 0.0 true)
    (`KismetSystemLibrary.MoveComponentTo` _button (`KismetMathLibrary.MakeVector` (- (.x (.location _returnvalue)) 1.5) (.y (.location _returnvalue)) (.z (.location _returnvalue))) (.rotation _returnvalue) false false 0.5)
    (`KismetSystemLibrary.Delay` 0.6)
    (`KismetSystemLibrary.MoveComponentTo` _button_2 (`KismetMathLibrary.MakeVector` (+ (.x (.location _returnvalue_2)) 1.5) (.y (.location _returnvalue_2)) (.z (.location _returnvalue_2))) (.rotation _returnvalue_2) false false 0.5)
    (`KismetSystemLibrary.Delay` 0.6)
    (bind _output_get_2 (set `self.isActivated` false))
    (`self.UpdateValueRender` (`KismetTextLibrary.Conv_BoolToText` _output_get_2))))

(fn `UserConstructionScript`)