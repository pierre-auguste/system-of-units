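; VR rotary button actor that a player grabs and twists with a motion controller to set a numeric value.
; Pickup records the controller's starting roll, registers with the VR pawn and opens a Tick gate.
; While held, roll change rotates the button, snaps the hand mesh onto it, updates the readout and messages ButtonOwner.
; Drop closes the gate, stores the value and resets the hand mesh.
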(event `self.ReceiveTick`
  (params (DeltaSeconds :type "Float (single-precision)"))
  (`/Engine/EditorBlueprintResources/StandardMacros.Gate` true :!label _label
    (:`Exit`
      (`self.Grabbing`))))

(event `/Game/SOU/Blueprints/Interfaces/SOU_PickupsInterface.Pickup`
  (params (MotionControlle :type "MotionControllerComponent Object Reference") (AttacheTo :type "SceneComponent Object Reference"))
  (`self.SetMotionController` MotionControlle)
  (goto _label :!via `Open`))

(event `/Game/SOU/Blueprints/Interfaces/SOU_PickupsInterface.Drop`
  (`|ExecutionSequence`
    (:`then_0`
      (goto _label :!via `Close`))
    (:`then_1`
      (bind _mc_aim_rotation (`self.GetControllerRotation`))
      (set `self.ButtonValue` (`self.GetActualValue` _mc_aim_rotation))
      (`SceneComponent.K2_SetRelativeLocationAndRotation` :`self` (`self.HandMesh`) :`bTeleport` true)
      (set `self.MotionController` null))))

(fn `GetControllerRotation`
  (returns (`MC AIM Rotation` :type "Float (single-precision)"))
  (locals (MC_Rotation :type "Rotator Structure"))
  (bind _mc_rotation_roll (`KismetMathLibrary.BreakRotator` (`local.MC_Rotation`)))
  (switch `name` (`MotionControllerComponent.MotionSource` (`self.MotionController`))
    (:`Default`
      (bind _motioncontrollerdata (`HeadMountedDisplayFunctionLibrary.GetMotionControllerData` null "Left"))
      (set `local.MC_Rotation` (`KismetMathLibrary.Quat_Rotator` (`.AimRotation` (break `XRMotionControllerData` _motioncontrollerdata)))))
    (:`Right`
      (bind _motioncontrollerdata_2 (`HeadMountedDisplayFunctionLibrary.GetMotionControllerData` null "Right"))
      (set `local.MC_Rotation` (`KismetMathLibrary.Quat_Rotator` (`.AimRotation` (break `XRMotionControllerData` _motioncontrollerdata_2))))))
  (return _mc_rotation_roll))

(fn `UserConstructionScript`
  (`parent.UserConstructionScript`)
  ;[1 0 0] ???
  (`PrimitiveComponent.SetCollisionResponseToChannel` (`self.Button`) "ECC_GameTraceChannel1" "ECR_Overlap"))